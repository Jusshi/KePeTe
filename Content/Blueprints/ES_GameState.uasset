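; Game state Blueprint that runs a timed escape and respawns the player when time runs out.
; StartEscape loads the countdown from EscapeTime and activates it, and Tick decrements it until it reaches zero.
; TimeOut then stops the timer, prints a message and destroys the player's pawn.
; After a short delay, it spawns a new PlayerCharacter at a PlayerStart and has the player controller possess it.
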(event Custom|TimeOut
  (Utilities|FlowControl|Sequence
    (:then_0
      (Development|PrintString "Time Is Up")
      (Variables|Default|SetescapeActive false)
      (Variables|Default|SetTimeRemaining 0.0))
    (:then_1
      (Actor|DestroyActor (Game|Player|GetPlayerPawn 0))
      (bind _returnvalue (Actor|GetActorOfClass "/Script/Engine.PlayerStart"))
      (Utilities|FlowControl|Delay 2.0)
      (bind _returnvalue_2 (Game|SpawnActorfromClass "/Game/Blueprints/PlayerCharacter.PlayerCharacter_C" (Transformation|GetActorTransform _returnvalue) "Undefined" 0 0))
      (Pawn|Possess (Game|GetPlayerController 0) _returnvalue_2))))

(event EventBeginPlay)

(event EventTick
  (params (DeltaSeconds :type Float%20%28single-precision%29))
  (if (Variables|Default|GetescapeActive)
    (bind _output_get (Variables|Default|SetTimeRemaining (- (Variables|Default|GetTimeRemaining) DeltaSeconds)))
    (if (<= _output_get 0.0)
      (CallFunction|TimeOut))))

(fn ConstructionScript)

(fn StartEscape
  (Variables|Default|SetTimeRemaining (Variables|Default|GetEscapeTime))
  (Variables|Default|SetescapeActive true))