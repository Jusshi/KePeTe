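; Surveillance camera actor that tracks the player inside its detection cone and dispatches an alarm.
; Cone overlap events set or clear DetectedPlayer for actors tagged Player.
; A dynamic decal material shows the camera state as green for seeking, yellow for analyzing and red for imminent alarm.
; State changes and alarm timing are not computed in this graph, which only responds through OnStateChange and OnRaiseAlarm.
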(event OnComponentBeginOverlap(SurveillanceCone)
  (params (OverlappedComponent :type Primitive%20Component%20Object%20Reference) (OtherActor :type Actor%20Object%20Reference) (OtherComp :type Primitive%20Component%20Object%20Reference) (OtherBodyIndex :type Integer) (bFromSweep :type Boolean) (SweepResult :type Hit%20Result%20Structure%20%28by%20ref%29))
  (if (Actor|ActorHasTag OtherActor "Player")
    (Variables|Default|SetdetectedPlayer OtherActor)))

(event OnComponentEndOverlap(SurveillanceCone)
  (params (OverlappedComponent :type Primitive%20Component%20Object%20Reference) (OtherActor :type Actor%20Object%20Reference) (OtherComp :type Primitive%20Component%20Object%20Reference) (OtherBodyIndex :type Integer))
  (if (Actor|ActorHasTag OtherActor "Player")
    (Variables|Default|SetdetectedPlayer 0)))

(event EventBeginPlay
  (bind _returnvalue (Rendering|Material|CreateDynamicMaterialInstance "/Game/SurveillanceCamera/AreaMaterial.AreaMaterial" "None" "None" :!class /Script/Engine.KismetMaterialLibrary))
  (bind _output_get (Variables|Default|SetDecalMaterial _returnvalue))
  (Rendering|Components|Decal|SetDecalMaterial (Variables|Default|GetDecal) _output_get)
  (Rendering|Material|SetVectorParameterValue (Variables|Default|GetDecalMaterial) "Color" "(R=0.000000,G=0.520000,B=0.039207,A=1.000000)" :!class /Script/Engine.MaterialInstanceDynamic))

(event Collision|EventActorBeginOverlap
  (params (OtherActor :type Actor%20Object%20Reference)))

(event EventTick
  (params (DeltaSeconds :type Float%20%28single-precision%29)))

(event EventOnRaiseAlarm
  (Development|PrintString "Alarm")
  (Default|CallAlarmDispatch))

(event EventOnStateChange
  (params (newState :type CameraState%20Enum :default "kSeeking"))
  (switch Utilities|FlowControl|Switch|SwitchonCameraState newState
    (:kSeeking
      (Rendering|Material|SetVectorParameterValue (Variables|Default|GetDecalMaterial) "Color" "(R=0.000000,G=0.520000,B=0.039207,A=1.000000)" :!class /Script/Engine.MaterialInstanceDynamic))
    (:kAnalyzing
      (Rendering|Material|SetVectorParameterValue (Variables|Default|GetDecalMaterial) "Color" "(R=0.944207,G=1.000000,B=0.000000,A=1.000000)" :!class /Script/Engine.MaterialInstanceDynamic))
    (:kAlarm
      (Rendering|Material|SetVectorParameterValue (Variables|Default|GetDecalMaterial) "Color" "(R=1.000000,G=0.000000,B=0.011734,A=1.000000)" :!class /Script/Engine.MaterialInstanceDynamic))))

(fn ConstructionScript)